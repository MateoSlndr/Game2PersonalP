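; A spawner actor that places one randomly chosen obstacle in the level when play begins.
; On BeginPlay it rolls a random integer stored in ObstacleType, then a chain of equality branches selects one of four SpawnActor calls.
; Each spawn uses the root component's world transform, so the obstacle appears at the spawner's own position and orientation.
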(event `self.ReceiveBeginPlay`
  (set `self.ObstacleType` 0)
  (bind _output_get (set `self.ObstacleType` (`KismetMathLibrary.RandomIntegerInRange` 0 3)))
  (if (== 0 _output_get)
    (`|SpawnActorFromClass` "/Game/Blueprints/BP_Obstacles.BP_Obstacles_C" (`SceneComponent.K2_GetComponentToWorld` (`self.DefaultSceneRoot`)) "Undefined" "MultiplyWithRoot" null null)
    (elif (== 1 _output_get)
      (`|SpawnActorFromClass` "/Game/Blueprints/BP_Obstacles1.BP_Obstacles1_C" (`SceneComponent.K2_GetComponentToWorld` (`self.DefaultSceneRoot`)) "Undefined" "MultiplyWithRoot" null null)
      (elif (== 2 _output_get)
        (`|SpawnActorFromClass` "/Game/Blueprints/BP_Obstacles2.BP_Obstacles2_C" (`SceneComponent.K2_GetComponentToWorld` (`self.DefaultSceneRoot`)) "Undefined" "MultiplyWithRoot" null null)
        (elif (== 3 _output_get)
          (`|SpawnActorFromClass` "/Game/Blueprints/BP_Obstacles3.BP_Obstacles3_C" (`SceneComponent.K2_GetComponentToWorld` (`self.DefaultSceneRoot`)) "Undefined" "MultiplyWithRoot" null null))))))

(fn `UserConstructionScript`)