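; BP_MovingLight is an actor that repeatedly slides its root component along the X axis.
; A timeline starts on BeginPlay and each update sets the root's X to the track value times 200, taking Y and Z from the Cube's world location.
; The update also feeds a 1.5-second Delay, which re-sets the root to its current location and restarts the timeline, forming the loop.
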(event `self.ReceiveBeginPlay`
  (bind (_returnvalue_x _returnvalue_y _returnvalue_z) (`KismetMathLibrary.BreakVector` (`SceneComponent.K2_GetComponentLocation` (`self.Cube`))))
  (bind (_direction _newtrack_0) (`Timeline|Timeline` :!label _label)
    (:`Update`
      (`SceneComponent.K2_SetRelativeLocation` (`self.DefaultSceneRoot`) (`KismetMathLibrary.MakeVector` (* _newtrack_0 200.0) _returnvalue_y _returnvalue_z) false false)
      (`KismetSystemLibrary.Delay` 1.5)
      (`SceneComponent.K2_SetWorldLocation` (`self.DefaultSceneRoot`) (`SceneComponent.K2_GetComponentLocation` (`self.DefaultSceneRoot`)) false false)
      (goto _label :!via `PlayFromStart`))))

(fn `UserConstructionScript`)